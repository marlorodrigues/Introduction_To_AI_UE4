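; Patrol path actor for enemy AI that turns an array of placed point actors into a visible route.
; The construction script builds a spline through the actors' world locations, with linear segments and an optional closed loop.
; It adds numbered text labels above each point.
; ShowPatrol unhides the point actors; otherwise the path hides itself and destroys stored labels before rebuilding, with no active runtime logic.
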(fn `UserConstructionScript`
  (locals (`LOCAL Point Location` :type "Array of Vector Structure") (`Local Spline Points Index` :type "Array of Integer") (`LOCAL Text Render Point` :type "TextRenderComponent Object Reference") (`LOCAL Text Render Point Text` :type Text) (`Local Text Render Point Num` :type Integer))
  (bind _patrol_points (`self.Patrol Points`))
  (bind _local_spline_points_index (`local.Local Spline Points Index`))
  (bind _spline (`self.Spline`))
  (bind _loop (`self.Loop`))
  (bind _spline_2 (`self.Spline`))
  (if (`self.Show Patrol`)
    (for _array_element _patrol_points
      (`self.SetActorHiddenInGame` _array_element false))
    (else
      (for _ _patrol_points
        (`self.SetActorHiddenInGame` true))
      (for _array_element_2 (`self.Text Render Points`)
        (`ActorComponent.K2_DestroyComponent` _array_element_2))))
  (`SplineComponent.SetSplinePoints` (`self.Spline`) (`local.LOCAL Point Location`) "World" true)
  (for _array_element_3 (`self.Patrol Points`)
    (`KismetArrayLibrary.Array_Add` (`local.LOCAL Point Location`) (`self.K2_GetActorLocation` _array_element_3)))
  (`SplineComponent.SetSplinePoints` _spline_2 (`local.LOCAL Point Location`) "World" true)
  (`KismetArrayLibrary.Array_Resize` _local_spline_points_index (`SplineComponent.GetNumberOfSplinePoints` _spline_2))
  (for (_ _array_index) _local_spline_points_index
    (`SplineComponent.SetSplinePointType` _spline _array_index "Linear" true))
  (if _loop
    (`SplineComponent.SetClosedLoop` _spline _loop true))
  (for _array_element_4 (`local.LOCAL Point Location`)
    (bind _returnvalue (`AddComponent|NODE_AddTextRenderComponent-0` :`bManualAttachment` true :`RelativeTransform` (`KismetMathLibrary.Conv_VectorToTransform` (`KismetMathLibrary.MakeVector` (.x _array_element_4) (.y _array_element_4) (+ (.z _array_element_4) 108.0)))))
    (`KismetArrayLibrary.Array_Add` (`self.Text Render Points`) _returnvalue)
    (bind _output_get (set `local.LOCAL Text Render Point` _returnvalue))
    (`TextRenderComponent.K2_SetText` _output_get (`local.LOCAL Text Render Point Text`))
    (bind _output_get_2 (set `local.Local Text Render Point Num` (+ (`local.Local Text Render Point Num`) 1)))
    (set `local.LOCAL Text Render Point Text` (`KismetTextLibrary.Conv_IntToText` _output_get_2))))