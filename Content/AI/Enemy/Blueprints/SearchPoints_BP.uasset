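; Enemy AI search point actor that holds a configurable number of sub-points, presumably locations for enemies to search.
; The construction script resizes the location array to the point count and adds a TargetPoint child actor component for each point.
; It then moves each stored component to its relative location from the array, slightly raised; an author note requires all points to be on the navmesh.
; The event graph has no logic.
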(fn `UserConstructionScript`
  (locals (`LOCAL Count Points` :type Integer))
  (bind _number_of_search_points (`self.Number Of Search Points`))
  (bind (_returnvalue_location _returnvalue_rotation _returnvalue_scale) (`KismetMathLibrary.BreakTransform` (`self.GetTransform` self)))
  (`KismetArrayLibrary.Array_Resize` (`self.Search Subpoints Locations`) _number_of_search_points)
  (while (not (== _number_of_search_points (`local.LOCAL Count Points`)))
    (set `local.LOCAL Count Points` (+ (`local.LOCAL Count Points`) 1))
    (bind _returnvalue (`AddComponent|NODE_AddChildActorComponent-0` :`RelativeTransform` (`KismetMathLibrary.MakeTransform` (`KismetMathLibrary.MakeVector` (+ (.x _returnvalue_location) 60.0) (.y _returnvalue_location) (+ (.z _returnvalue_location) 20.0)) _returnvalue_rotation _returnvalue_scale)))
    (`ChildActorComponent.SetChildActorClass` _returnvalue "/Script/Engine.TargetPoint")
    (`KismetArrayLibrary.Array_Add` (`self.Search Subpoints Ref`) _returnvalue))
  (for (_array_element _array_index) (`self.Search Subpoints Ref`)
    (bind (_output_x _output_y _output_z) (`KismetMathLibrary.BreakVector` (`|GetArrayItem` (`self.Search Subpoints Locations`) _array_index)))
    (`SceneComponent.K2_SetRelativeTransform` _array_element (`KismetMathLibrary.MakeTransform` (`KismetMathLibrary.MakeVector` _output_x _output_y (+ _output_z 10.0))) false false) ; ALL POINT MUST BE ON NAVMESH
  ))